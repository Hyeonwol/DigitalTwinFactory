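; BP_ConveyorEngine is an item actor that rides a conveyor path's spline and counts as one produced item when it reaches the end.
; InitializeEngine assigns the path and start distance, then Tick advances the distance by speed and delta time.
; UpdateEnginePosition snaps location to the spline and optionally smooths rotation toward its direction.
; Past the spline's end, it calls CompleteOneItem once on every BP_ProductionManager and destroys itself after a short delay.
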(event `self.ReceiveTick`
  (params (DeltaSeconds :type "Float (single-precision)"))
  (bind _conveyorpath (`self.ConveyorPath`))
  (`/Engine/EditorBlueprintResources/StandardMacros.IsValid` _conveyorpath
    (:`Is Valid`
      (if (`self.IsMoving`)
        (bind _output_get (set `self.DistanceAlongSpline` (+ (* (`self.MoveSpeed`) DeltaSeconds) (`self.DistanceAlongSpline`))))
        (`self.UpdateEnginePosition`)
        (if (and (> _output_get (`SplineComponent.GetSplineLength` (`/Game/Blueprints/Conveyor/BP_ConveyorPath.ConveyorSpline` _conveyorpath))) (not (`self.HasCompletedPath`)))
          (set `self.HasCompletedPath` true)
          (bind _outactors (`GameplayStatics.GetAllActorsOfClass` "/Game/Blueprints/Conveyor/UI/BP_ProductionManager.BP_ProductionManager_C"))
          (for _array_element _outactors
            (`/Game/Blueprints/Conveyor/UI/BP_ProductionManager.CompleteOneItem` _array_element))
          (`KismetSystemLibrary.Delay` 0.5)
          (`self.K2_DestroyActor`))))))

(fn `InitializeEngine`
  (params (ConveyorPath :type "/Game/Blueprints/Conveyor/BP_ConveyorPath Object Reference") (StartDistance :type "Float (double-precision)"))
  (set `self.ConveyorPath` ConveyorPath)
  (set `self.DistanceAlongSpline` StartDistance)
  (set `self.IsMoving` true)
  (`self.UpdateEnginePosition`))

(fn `UpdateEnginePosition`
  (bind _conveyorpath (`self.ConveyorPath`))
  (`/Engine/EditorBlueprintResources/StandardMacros.IsValid` _conveyorpath
    (:`Is Valid`
      (bind _conveyorspline (`/Game/Blueprints/Conveyor/BP_ConveyorPath.ConveyorSpline` _conveyorpath)
        (:`then`
          (`self.K2_SetActorLocation` (`SplineComponent.GetLocationAtDistanceAlongSpline` _conveyorspline (`self.DistanceAlongSpline`) "World"))
          (if (`self.RotateToSpline`)
            (`self.K2_SetActorRotation` (`KismetMathLibrary.RInterpTo` (`self.K2_GetActorRotation`) (`KismetMathLibrary.MakeRotFromX` (`SplineComponent.GetDirectionAtDistanceAlongSpline` _conveyorspline (`self.DistanceAlongSpline`) "World")) (`GameplayStatics.GetWorldDeltaSeconds`) 8.0))))
        (:`else`)))))

(fn `UserConstructionScript`)