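; Conveyor robot arm actor that turns toward a passing BP_ConveyorEngine and plays a looping arm animation while the engine is in its DetectionZone.
; Overlap begin locks onto one engine and picks its left or right contact point by ArmPosition, which Tick tracks by interpolating the whole actor's rotation.
; Any overlap end stops the animation and eases back to the initial rotation through a timeline.
; Pivot-only rotation nodes remain but never run.
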(event `Start Reset Rotation`
  (`Timeline|Rotation Reset Timeline` :!via `PlayFromStart`
    (:`Update`
      (`self.K2_SetActorRotation` (`KismetMathLibrary.RInterpTo` (`self.K2_GetActorRotation`) (`self.InitialRotation`) (`GameplayStatics.GetWorldDeltaSeconds`) 5.0)))))

(event `self.ReceiveBeginPlay`
  (set `self.InitialRotation` (`self.K2_GetActorRotation`)))

(event `self.ReceiveTick`
  (params (DeltaSeconds :type "Float (single-precision)"))
  (bind _enginetargetpoint (`self.EngineTargetPoint`))
  (if (`self.IsProcessing`)
    (`/Engine/EditorBlueprintResources/StandardMacros.IsValid` (`self.CurrentEngine`)
      (:`Is Valid`
        (`/Engine/EditorBlueprintResources/StandardMacros.IsValid` _enginetargetpoint
          (:`Is Valid`
            (`self.K2_SetActorRotation` (`KismetMathLibrary.RInterpTo` (`self.K2_GetActorRotation`) (`KismetMathLibrary.MakeRotFromX` (- (`SceneComponent.K2_GetComponentLocation` _enginetargetpoint) (`SceneComponent.K2_GetComponentLocation` (`self.ArmEnd`)))) DeltaSeconds 5.0))))))))

(event `self.DetectionZone.OnComponentBeginOverlap`
  (params (OverlappedComponent :type "PrimitiveComponent Object Reference") (OtherActor :type "Actor Object Reference") (OtherComp :type "PrimitiveComponent Object Reference") (OtherBodyIndex :type Integer) (bFromSweep :type Boolean) (SweepResult :type "HitResult Structure (by ref)"))
  (bind (_asbp_conveyor_engine _bsuccess) (cast `/Game/Blueprints/Conveyor/BP_ConveyorEngine` OtherActor :!pure true))
  (if _bsuccess
    (`self.ProcessEngine` _asbp_conveyor_engine)))

(event `self.DetectionZone.OnComponentEndOverlap`
  (params (OverlappedComponent :type "PrimitiveComponent Object Reference") (OtherActor :type "Actor Object Reference") (OtherComp :type "PrimitiveComponent Object Reference") (OtherBodyIndex :type Integer))
  (`self.ResetRobot`))

(fn `ProcessEngine`
  (params (OverlappedEngine :type "/Game/Blueprints/Conveyor/BP_ConveyorEngine Object Reference"))
  (if (`self.IsProcessing`)
    (return)
    (else
      (bind _output_get (set `self.CurrentEngine` OverlappedEngine))
      (set `self.IsProcessing` true)
      (if (`|EnumEquality` (`self.ArmPosition`) "NewEnumerator0")
        (set `self.EngineTargetPoint` (`/Game/Blueprints/Conveyor/BP_ConveyorEngine.LeftContactPoint` _output_get))
        (else
          (set `self.EngineTargetPoint` (`/Game/Blueprints/Conveyor/BP_ConveyorEngine.RightContactPoint` _output_get))))
      (`SkeletalMeshComponent.PlayAnimation` (`self.ArmComponent`) "/Game/Meshes/Robot/M_RobotArm.M_RobotArm" true))))

(fn `ResetRobot`
  (bind _armcomponent (`self.ArmComponent`))
  (set `self.IsProcessing` false)
  (set `self.CurrentEngine` null)
  (set `self.EngineTargetPoint` null)
  (`SkeletalMeshComponent.Stop` _armcomponent)
  (`SkeletalMeshComponent.SetAnimationMode` _armcomponent "AnimationSingleNode" true)
  (`self.Start Reset Rotation`))

(fn `UserConstructionScript`)