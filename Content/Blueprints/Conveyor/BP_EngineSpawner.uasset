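; BP_EngineSpawner is an actor that feeds engines onto a conveyor path.
; On BeginPlay, if a target path is valid and spawning is enabled, it spawns one engine immediately and starts a looping timer at the spawn interval.
; Each spawn creates the configured engine class at the start of the path's spline and initializes it with that path at zero distance.
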(event `self.ReceiveBeginPlay`
  (`/Engine/EditorBlueprintResources/StandardMacros.IsValid` (`self.TargetConveyorPath`)
    (:`Is Valid`
      (if (`self.IsSpawning`)
        (`self.SpawnEngine`)
        (`KismetSystemLibrary.K2_SetTimer` null "SpawnEngine" (`self.SpawnInterval`) true)))))

(fn `SpawnEngine`
  (bind _targetconveyorpath (`self.TargetConveyorPath`))
  (`/Engine/EditorBlueprintResources/StandardMacros.IsValid` _targetconveyorpath
    (:`Is Valid`
      (bind _returnvalue (`|SpawnActorFromClass` (`self.EngineClass`) (`KismetMathLibrary.MakeTransform` (`SplineComponent.GetLocationAtDistanceAlongSpline` (`/Game/Blueprints/Conveyor/BP_ConveyorPath.ConveyorSpline` _targetconveyorpath) 0.0 "World")) "Undefined" "MultiplyWithRoot" null null))
      (`/Game/Blueprints/Conveyor/BP_ConveyorEngine.InitializeEngine` _returnvalue (`self.TargetConveyorPath`) 0.0))))

(fn `UserConstructionScript`)