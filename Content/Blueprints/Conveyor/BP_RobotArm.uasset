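; BP_RobotArm is a conveyor robot arm actor that turns toward an engine and plays a looping animation while processing it.
; ProcessEngine claims one engine at a time, choosing its left or right contact point from ArmPosition.
; Tick smoothly yaws the whole actor along the flattened direction from ArmEnd to that point.
; ResetRobot releases the matching engine, stops the animation and runs a timeline that interpolates back toward the starting rotation.
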(event `Start Reset Rotation`
  (`Timeline|Rotation Reset Timeline` :!via `PlayFromStart`
    (:`Update`
      (`self.K2_SetActorRotation` (`KismetMathLibrary.RInterpTo` (`self.K2_GetActorRotation`) (`self.InitialRotation`) (`GameplayStatics.GetWorldDeltaSeconds`) 5.0)))))

(event `self.ReceiveBeginPlay`
  (set `self.InitialRotation` (`self.K2_GetActorRotation`)))

(event `self.ReceiveTick`
  (params (DeltaSeconds :type "Float (single-precision)"))
  (bind _returnvalue (`self.K2_GetActorRotation`))
  (bind _enginetargetpoint (`self.EngineTargetPoint`))
  (bind (_returnvalue_x _returnvalue_y) (`KismetMathLibrary.BreakVector` (- (`SceneComponent.K2_GetComponentLocation` _enginetargetpoint) (`SceneComponent.K2_GetComponentLocation` (`self.ArmEnd`)))))
  (if (`self.IsProcessing`)
    (`/Engine/EditorBlueprintResources/StandardMacros.IsValid` (`self.CurrentEngine`)
      (:`Is Valid`
        (`/Engine/EditorBlueprintResources/StandardMacros.IsValid` _enginetargetpoint
          (:`Is Valid`
            (`self.K2_SetActorRotation` (`KismetMathLibrary.RInterpTo` _returnvalue (`KismetMathLibrary.MakeRotator` (.roll _returnvalue) (.pitch _returnvalue) (.yaw (`KismetMathLibrary.MakeRotFromX` (`KismetMathLibrary.Normal` (`KismetMathLibrary.MakeVector` _returnvalue_x _returnvalue_y))))) DeltaSeconds 5.0))))))))

(fn `ProcessEngine`
  (params (TargetEngine :type "/Game/Blueprints/Conveyor/BP_ConveyorEngine Object Reference"))
  (if (`self.IsProcessing`)
    (return)
    (else
      (bind _output_get (set `self.CurrentEngine` TargetEngine))
      (set `self.IsProcessing` true)
      (if (`|EnumEquality` (`self.ArmPosition`) "NewEnumerator0")
        (set `self.EngineTargetPoint` (`/Game/Blueprints/Conveyor/BP_ConveyorEngine.LeftContactPoint` _output_get))
        (else
          (set `self.EngineTargetPoint` (`/Game/Blueprints/Conveyor/BP_ConveyorEngine.RightContactPoint` _output_get))))
      (`SkeletalMeshComponent.PlayAnimation` (`self.ArmComponent`) "/Game/Meshes/Robot/M_RobotArm.M_RobotArm" true))))

(fn `ResetRobot`
  (params (TargetEngine :type "/Game/Blueprints/Conveyor/BP_ConveyorEngine Object Reference"))
  (bind _armcomponent (`self.ArmComponent`))
  (if (== (`self.CurrentEngine`) TargetEngine)
    (set `self.IsProcessing` false)
    (set `self.CurrentEngine` null)
    (set `self.EngineTargetPoint` null)
    (`SkeletalMeshComponent.Stop` _armcomponent)
    (`SkeletalMeshComponent.SetAnimationMode` _armcomponent "AnimationSingleNode" true)
    (`self.Start Reset Rotation`)))

(fn `UserConstructionScript`)