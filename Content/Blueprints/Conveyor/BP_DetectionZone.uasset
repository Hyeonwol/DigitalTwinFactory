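; BP_DetectionZone is a conveyor trigger volume that detects engines and notifies an assigned robot arm.
; Its DetectionZone component's overlap events filter for BP_ConveyorEngine actors and forward them to TargetRobotArm, if that reference is valid.
; Begin overlap calls ProcessEngine on the arm with the engine, and end overlap calls ResetRobot with it.
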(event `self.DetectionZone.OnComponentBeginOverlap`
  (params (OverlappedComponent :type "PrimitiveComponent Object Reference") (OtherActor :type "Actor Object Reference") (OtherComp :type "PrimitiveComponent Object Reference") (OtherBodyIndex :type Integer) (bFromSweep :type Boolean) (SweepResult :type "HitResult Structure (by ref)"))
  (bind (_asbp_conveyor_engine _bsuccess) (cast `/Game/Blueprints/Conveyor/BP_ConveyorEngine` OtherActor :!pure true))
  (bind _targetrobotarm (`self.TargetRobotArm`))
  (if _bsuccess
    (`/Engine/EditorBlueprintResources/StandardMacros.IsValid` _targetrobotarm
      (:`Is Valid`
        (`/Game/Blueprints/Conveyor/BP_RobotArm.ProcessEngine` _targetrobotarm _asbp_conveyor_engine)))))

(event `self.DetectionZone.OnComponentEndOverlap`
  (params (OverlappedComponent :type "PrimitiveComponent Object Reference") (OtherActor :type "Actor Object Reference") (OtherComp :type "PrimitiveComponent Object Reference") (OtherBodyIndex :type Integer))
  (bind (_asbp_conveyor_engine _bsuccess) (cast `/Game/Blueprints/Conveyor/BP_ConveyorEngine` OtherActor :!pure true))
  (bind _targetrobotarm (`self.TargetRobotArm`))
  (if _bsuccess
    (`/Engine/EditorBlueprintResources/StandardMacros.IsValid` _targetrobotarm
      (:`Is Valid`
        (`/Game/Blueprints/Conveyor/BP_RobotArm.ResetRobot` _targetrobotarm _asbp_conveyor_engine)))))

(fn `UserConstructionScript`)