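; Anim notify state that plays the welding contact sound on a BP_RobotArm for the duration of the notify window in its animation.
; On begin, it spawns the arm's ContactSound at its EffectLocation and stores the audio component on the arm.
; On end, it stops that component if valid and clears the reference.
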(fn `Received_NotifyBegin`
  (params (MeshComp :type "SkeletalMeshComponent Object Reference") (Animation :type "AnimSequenceBase Object Reference") (TotalDuration :type "Float (single-precision)") (EventReference :type "AnimNotifyEventReference Structure (by ref)"))
  (returns (ReturnValue :type Boolean))
  (bind _asbp_robot_arm (cast `/Game/Blueprints/Conveyor/BP_RobotArm` (`ActorComponent.GetOwner` MeshComp) :!pure true))
  (bind _returnvalue (`GameplayStatics.SpawnSoundAtLocation` _asbp_robot_arm (`/Game/Blueprints/Conveyor/BP_RobotArm.ContactSound` _asbp_robot_arm) (`/Game/Blueprints/Conveyor/BP_RobotArm.EffectLocation` _asbp_robot_arm) (struct) 1.0 1.0 0.0 null null))
  (set `/Game/Blueprints/Conveyor/BP_RobotArm.WeldingAudioComponent` _returnvalue _asbp_robot_arm)
  (return false))

(fn `Received_NotifyEnd`
  (params (MeshComp :type "SkeletalMeshComponent Object Reference") (Animation :type "AnimSequenceBase Object Reference") (EventReference :type "AnimNotifyEventReference Structure (by ref)"))
  (returns (ReturnValue :type Boolean))
  (bind _asbp_robot_arm (cast `/Game/Blueprints/Conveyor/BP_RobotArm` (`ActorComponent.GetOwner` MeshComp) :!pure true))
  (bind _weldingaudiocomponent (`/Game/Blueprints/Conveyor/BP_RobotArm.WeldingAudioComponent` _asbp_robot_arm))
  (`/Engine/EditorBlueprintResources/StandardMacros.IsValid` _weldingaudiocomponent
    (:`Is Valid`
      (`AudioComponent.Stop` _weldingaudiocomponent)
      (set `/Game/Blueprints/Conveyor/BP_RobotArm.WeldingAudioComponent` null _asbp_robot_arm)
      (return false))))